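; GI_BaseInstance is a Game Instance Blueprint that holds the game's options and persists them through SG_Options save objects.
; UpdateGameOptions stores incoming options and immediately writes them to the OptionsSlot save slot in a newly created object.
; LoadSaveOptions reads that slot, or takes a new object's defaults without saving when none exists, printing which path ran.
; SaveOptions is empty, and a duplicate save chain is left unconnected.
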(event Custom|UpdateGameOptions
  (params (InOptions :type STRUCT%20Options%20Structure))
  (Variables|Default|SetGameOptions InOptions)
  (bind _returnvalue (SaveGame|CreateSaveGameObject "/Game/Blueprints/Classes/SG_Options.SG_Options_C"))
  (Variables|/Game/Blueprints/Classes/SG_Options.SG_Options_C|SetOptions _returnvalue (Variables|Default|GetGameOptions))
  (SaveGame|SaveGametoSlot _returnvalue "OptionsSlot"))

(event Custom|SaveOptions)

(event Custom|LoadSaveOptions
  (bind _returnvalue (SaveGame|DoesSaveGameExist "OptionsSlot"))
  (if _returnvalue
    (bind _returnvalue_2 (SaveGame|LoadGamefromSlot "OptionsSlot"))
    (bind _assg_options (Utilities|Casting|CastToSG_Options _returnvalue_2))
    (Variables|Default|SetGameOptions (Variables|/Game/Blueprints/Classes/SG_Options.SG_Options_C|GetOptions _assg_options))
    (Development|PrintString "OPTIONS LOADED FROM STORAGE" true true "(R=0.000000,G=0.660000,B=1.000000,A=1.000000)" 15.0)
    (else
      (bind _returnvalue_3 (SaveGame|CreateSaveGameObject "/Game/Blueprints/Classes/SG_Options.SG_Options_C"))
      (Variables|Default|SetGameOptions (Variables|/Game/Blueprints/Classes/SG_Options.SG_Options_C|GetOptions _returnvalue_3))
      (Development|PrintString "NEW SAVED OPTIONS OBJECT CREATED" true true "(R=0.000000,G=0.660000,B=1.000000,A=1.000000)" 15.0))))