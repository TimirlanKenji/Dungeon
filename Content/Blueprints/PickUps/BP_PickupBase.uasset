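; Base pickup Blueprint for collectibles that report to BP_ThirdPersonGameMode, registering on BeginPlay and signaling collection whenever the actor is destroyed.
; The ChangeState event destroys the actor, while the sphere overlap event has no logic here.
; The Construction Script configures the point light from color, intensity and attenuation variables and assigns a GUID string when ID is empty, exposed through GetID.
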(event OnComponentBeginOverlap(SphereColl)
  (params (OverlappedComponent :type Primitive%20Component%20Object%20Reference) (OtherActor :type Actor%20Object%20Reference) (OtherComp :type Primitive%20Component%20Object%20Reference) (OtherBodyIndex :type Integer) (bFromSweep :type Boolean) (SweepResult :type Hit%20Result%20Structure%20%28by%20ref%29)))

(event EventBeginPlay
  (Default|RegisterCollectible (.AsBP%20Third%20Person%20Game%20Mode (Utilities|Casting|CastToBP_ThirdPersonGameMode (Game|GetGameMode)))))

(event EventDestroyed
  (bind _asbp_third_person_game_mode (Utilities|Casting|CastToBP_ThirdPersonGameMode (Game|GetGameMode)))
  (Default|CollectibleCollected _asbp_third_person_game_mode))

(event EventTick
  (params (DeltaSeconds :type Float%20%28single-precision%29)))

(event EventChangeState
  (Actor|DestroyActor))

(fn ConstructionScript
  (bind _pointlight (Variables|Default|GetPointLight))
  ;[1 0.2581 0.7299] each object has its own ID
  (Utilities|FlowControl|Sequence
    (:then_0
      ;[0.2633 1 0.3058] Point Light Configure
      (Rendering|Components|Light|SetLightColor _pointlight (Variables|Default|GetLightColor) true)
      (Rendering|Components|Light|SetIntensity _pointlight (Variables|Default|GetLightIntensity))
      (Rendering|Lighting|SetAttenuationRadius _pointlight (Variables|Default|GetLightAttenuation)))
    (:then_1
      (if (Utilities|Enum|Equal(Enum) (Variables|Default|GetID) "")
        (Variables|Default|SetID (Class|MagicLeapARPinFunctionLibrary|ARPinIdtoString (Guid|NewGuid)))))))

(fn GetID
  (return (Variables|Default|GetID)))