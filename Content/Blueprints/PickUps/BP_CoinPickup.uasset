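; Coin pickup actor that counts toward the current coin total in BP_ThirdPersonGameMode and registers itself there as a collectible on BeginPlay.
; Any overlap with its sphere, with no check on the overlapping actor, increments CurrentCoin and destroys the coin.
; A ChangeState event destroys it without incrementing the count.
; Destroyed reports the coin's ID to the game mode through CollectibleCollected, whatever caused the destruction.
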(event OnComponentBeginOverlap(SphereColl)
  (params (OverlappedComponent :type Primitive%20Component%20Object%20Reference) (OtherActor :type Actor%20Object%20Reference) (OtherComp :type Primitive%20Component%20Object%20Reference) (OtherBodyIndex :type Integer) (bFromSweep :type Boolean) (SweepResult :type Hit%20Result%20Structure%20%28by%20ref%29))
  (bind _asbp_third_person_game_mode (Utilities|Casting|CastToBP_ThirdPersonGameMode (Game|GetGameMode)))
  (Variables|/Game/Blueprints/BP_ThirdPersonGameMode.BP_ThirdPersonGameMode_C|SetCurrentCoin _asbp_third_person_game_mode (+ (Variables|/Game/Blueprints/BP_ThirdPersonGameMode.BP_ThirdPersonGameMode_C|GetCurrentCoin _asbp_third_person_game_mode) 1))
  (Actor|DestroyActor))

(event EventBeginPlay
  (Default|RegisterCollectible (.AsBP%20Third%20Person%20Game%20Mode (Utilities|Casting|CastToBP_ThirdPersonGameMode (Game|GetGameMode)))))

(event EventDestroyed
  (bind _asbp_third_person_game_mode (Utilities|Casting|CastToBP_ThirdPersonGameMode (Game|GetGameMode)))
  (Default|CollectibleCollected _asbp_third_person_game_mode (Variables|Default|GetID)))

(event EventTick
  (params (DeltaSeconds :type Float%20%28single-precision%29)))

(event EventChangeState
  (Actor|DestroyActor))

(event Collision|EventActorBeginOverlap
  (params (OtherActor :type Actor%20Object%20Reference)))

(fn ConstructionScript
  (|CallParentFunction))