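; BP_FuelPickup is a pickup actor that refills the player's fuel.
; On overlap with BP_ThirdPersonCharacter, it adds a fixed amount to the character's PlayerFuel, prints the new value and destroys itself.
; The addition is not clamped, and BeginPlay, Tick and the construction script add no logic of their own.
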(event EventBeginPlay
  (|CallParentFunction) ; This node is disabled and will not be called.\nDrag off pins to build functionality.
)

(event Collision|EventActorBeginOverlap
  (params (OtherActor :type Actor%20Object%20Reference))
  (bind _asbp_third_person_character (Utilities|Casting|CastToBP_ThirdPersonCharacter OtherActor))
  (bind _output_get (Variables|/Game/Blueprints/BP_ThirdPersonCharacter.BP_ThirdPersonCharacter_C|SetPlayerFuel _asbp_third_person_character (+ (Variables|/Game/Blueprints/BP_ThirdPersonCharacter.BP_ThirdPersonCharacter_C|GetPlayerFuel _asbp_third_person_character) 0.25)))
  (Development|PrintString (Utilities|String|ToString(Float) _output_get) true false "(R=0.000000,G=1.000000,B=0.110761,A=1.000000)")
  (Actor|DestroyActor))

(event EventTick
  (params (DeltaSeconds :type Float%20%28single-precision%29))
  (|CallParentFunction DeltaSeconds) ; This node is disabled and will not be called.\nDrag off pins to build functionality.
)

(fn ConstructionScript
  (|CallParentFunction))