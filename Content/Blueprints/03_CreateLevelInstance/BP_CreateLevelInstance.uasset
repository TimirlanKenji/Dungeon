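; A trigger box actor that spawns streamed level sections at connector points when a Character overlaps it.
; ManageLevelInstance fires once, giving each available connector a random pick from five streaming levels and marking that connector unavailable.
; Each pick becomes a level instance named with the game mode's instance count, placed at the connector's transform, loaded and shown.
; CustomLevelReset frees the connectors and re-arms the trigger.
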(event OnComponentBeginOverlap(Box)
  (params (OverlappedComponent :type Primitive%20Component%20Object%20Reference) (OtherActor :type Actor%20Object%20Reference) (OtherComp :type Primitive%20Component%20Object%20Reference) (OtherBodyIndex :type Integer) (bFromSweep :type Boolean) (SweepResult :type Hit%20Result%20Structure%20%28by%20ref%29))
  (Utilities|Casting|CastToCharacter OtherActor)
  (CallFunction|ManageLevelInstance))

(event EventBeginPlay)

(fn ConstructionScript
  (Components|Box|SetBoxExtent (Variables|Default|GetBox) (Variables|Default|GetExtent) true))

(fn ManageLevelInstance
  (if (not (Variables|Default|GetOnce))
    (Variables|Default|SetOnce true)
    (bind _asbp_third_person_game_mode (Utilities|Casting|CastToBP_ThirdPersonGameMode (Game|GetGameMode)))
    (Variables|Default|SetGameMode _asbp_third_person_game_mode)
    (if (Utilities|Array|IsValidIndex (Variables|Default|GetCurConnector))
      (for _array_element (Variables|Default|GetCurConnector)
        (bind _output_get (LocalVariables|SetL_Con _array_element))
        (if (Variables|/Game/Blueprints/03_CreateLevelInstance/BP_Connection.BP_Connection_C|GetAvailable _output_get)
          (Variables|/Game/Blueprints/03_CreateLevelInstance/BP_Connection.BP_Connection_C|SetAvailable (LocalVariables|GetL_Con) false)
          (Variables|Default|SetLevelName (Utilities|Select :Index (Math|Random|RandomIntegerinRange 0 4) :Option%200 "Level_A" :Option%201 "Level_B" :Option%202 "Level_C" :Option%203 "Level_D" :Option%204 "Level_E"))
          (Utilities|IsValid (Class|GameplayStatics|GetStreamingLevel (Variables|Default|GetLevelName))
            (:Is%20Valid
              (bind _returnvalue (Class|LevelStreaming|CreateInstance (Class|GameplayStatics|GetStreamingLevel (Variables|Default|GetLevelName)) (Utilities|String|Append (Utilities|String|ToString(Name) (Variables|Default|GetLevelName)) "_" (Utilities|String|ToString(Integer) (Default|CountLevelInstances (Variables|Default|GetGameMode))))))
              (Variables|Default|SetInstance _returnvalue)
              (Utilities|Array|AddUnique (Variables|Default|GetInstances) (Variables|Default|GetInstance))
              (Variables|/Script/Engine.LevelStreaming|SetLevelTransform (Variables|Default|GetInstance) (Transformation|GetActorTransform (LocalVariables|GetL_Con)))
              (Variables|/Script/Engine.LevelStreaming|SetbShouldBeLoaded (Variables|Default|GetInstance) true)
              (Variables|/Script/Engine.LevelStreaming|SetbShouldBeVisible (Variables|Default|GetInstance) true))))))))

(fn CustomLevelReset
  (Utilities|FlowControl|Sequence
    (:then_0
      (if (Utilities|Array|IsValidIndex (Variables|Default|GetCurConnector))
        (for _array_element (Variables|Default|GetCurConnector)
          (Variables|/Game/Blueprints/03_CreateLevelInstance/BP_Connection.BP_Connection_C|SetAvailable _array_element true))))
    (:then_1
      (Variables|Default|SetOnce false))))