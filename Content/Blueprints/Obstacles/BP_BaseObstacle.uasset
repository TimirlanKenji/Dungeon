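; Base obstacle Blueprint that applies damage over time to the third-person player character while it overlaps the Box trigger.
; Begin overlap caches the character, copies Damage into its DamageSum and starts a short looping timer that repeatedly calls PlayerDamaged on it.
; End overlap resets PlayerInsideRadius and clears the timer.
; BeginPlay starts the same timer if that flag is already set.
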(event OnComponentBeginOverlap(Box)
  (params (OverlappedComponent :type Primitive%20Component%20Object%20Reference) (OtherActor :type Actor%20Object%20Reference) (OtherComp :type Primitive%20Component%20Object%20Reference) (OtherBodyIndex :type Integer) (bFromSweep :type Boolean) (SweepResult :type Hit%20Result%20Structure%20%28by%20ref%29))
  (bind _asbp_third_person_character (Utilities|Casting|CastToBP_ThirdPersonCharacter OtherActor))
  (Variables|Default|SetPlayerInsideRadius true)
  (Variables|/Game/Blueprints/BP_ThirdPersonCharacter.BP_ThirdPersonCharacter_C|SetDamageSum _asbp_third_person_character (Variables|Default|GetDamage))
  (bind _returnvalue (Utilities|Time|SetTimerbyEvent (delegate Custom|DOTEvent) 0.2 true))
  (Variables|Default|SetDOTTimerHandler _returnvalue))

(event OnComponentEndOverlap(Box)
  (params (OverlappedComponent :type Primitive%20Component%20Object%20Reference) (OtherActor :type Actor%20Object%20Reference) (OtherComp :type Primitive%20Component%20Object%20Reference) (OtherBodyIndex :type Integer))
  (Utilities|Casting|CastToBP_ThirdPersonCharacter OtherActor)
  (Variables|Default|SetPlayerInsideRadius false)
  (if (Utilities|Time|IsValidTimerHandle (Variables|Default|GetDOTTimerHandler))
    (Utilities|Time|ClearandInvalidateTimerbyHandle (Variables|Default|GetDOTTimerHandler))))

(event Custom|DOTEvent
  (Default|PlayerDamaged (stale OnComponentBeginOverlap(Box) _asbp_third_person_character)))

(event EventBeginPlay
  (if (Variables|Default|GetPlayerInsideRadius)
    (bind _returnvalue (Utilities|Time|SetTimerbyEvent (delegate Custom|DOTEvent) 0.2 true))
    (Variables|Default|SetDOTTimerHandler _returnvalue)))

(fn ConstructionScript)