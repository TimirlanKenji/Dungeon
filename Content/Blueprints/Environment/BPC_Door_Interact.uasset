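; Interactable door Blueprint that the player opens and closes with the Interact input while standing inside its trigger.
; Trigger overlaps by the player character enable or disable input on the actor and show or hide the EOnTheLeft prompt.
; Each Interact press alternates through a FlipFlop between OpenDoor and CloseDoor, which are not defined in this Blueprint's graphs.
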(event OnComponentBeginOverlap(Trigger)
  (params (OverlappedComponent :type Primitive%20Component%20Object%20Reference) (OtherActor :type Actor%20Object%20Reference) (OtherComp :type Primitive%20Component%20Object%20Reference) (OtherBodyIndex :type Integer) (bFromSweep :type Boolean) (SweepResult :type Hit%20Result%20Structure%20%28by%20ref%29))
  ;[1 1 1] Overlap- enable and disable Input
  (if (== OtherActor (Game|GetPlayerCharacter 0))
    (Input|EnableInput (Game|GetPlayerController 0))
    (Development|SetHiddeninGame (Variables|Default|GetE%20on%20the%20Left) false false)))

(event OnComponentEndOverlap(Trigger)
  (params (OverlappedComponent :type Primitive%20Component%20Object%20Reference) (OtherActor :type Actor%20Object%20Reference) (OtherComp :type Primitive%20Component%20Object%20Reference) (OtherBodyIndex :type Integer))
  ;[1 1 1] Overlap- enable and disable Input
  (if (== OtherActor (Game|GetPlayerCharacter 0))
    (Input|DisableInput (Game|GetPlayerController 0))
    (Development|SetHiddeninGame (Variables|Default|GetE%20on%20the%20Left) true false)))

(event Input|ActionEvents|InputActionInteract
  (params (Key :type Key%20Structure :default "None"))
  ;[0.06722 1 0] Interact logic
  (:Pressed
    (Utilities|FlowControl|FlipFlop
      (:A
        (CallFunction|OpenDoor))
      (:B
        (CallFunction|CloseDoor)))))

(fn ConstructionScript
  (|CallParentFunction))