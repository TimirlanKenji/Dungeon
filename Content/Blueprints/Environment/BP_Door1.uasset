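; Door actor that swings open when an actor overlaps its Trigger component.
; The overlapping actor's position in the door's local space picks the swing direction, so yaw heads to either side by a quarter turn.
; The SwingOpen timeline drives a rotation lerp against the door's current rotation while pinning its relative location.
; DoorOpen blocks retriggering once the swing starts; no closing logic exists.
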(event OnComponentBeginOverlap(Trigger)
  (params (OverlappedComponent :type Primitive%20Component%20Object%20Reference) (OtherActor :type Actor%20Object%20Reference) (OtherComp :type Primitive%20Component%20Object%20Reference) (OtherBodyIndex :type Integer) (bFromSweep :type Boolean) (SweepResult :type Hit%20Result%20Structure%20%28by%20ref%29))
  (if (not (Variables|Default|GetDoorOpen))
    (Variables|Default|SetOpen%20direction (> (.X (Math|Vector|BreakVector (Math|Vector|UnrotateVector (- (Transformation|GetActorLocation) (Transformation|GetActorLocation OtherActor)) (Transformation|GetActorRotation)))) 0.0))
    (bind _rotation (Timeline|SwingOpen PlayFromStart)
      (:Update
        (Transformation|SetRelativeLocationAndRotation (Variables|Default|GetDoor) "0, 0,333.000000" (Math|Rotator|Lerp(Rotator) (Math|Rotator|MakeRotator 0.0 0.0 (Math|Float|SelectFloat -9e+01 9e+01 (Variables|Default|GetOpen%20direction))) (Variables|/Script/Engine.SceneComponent|GetRelativeRotation (Variables|Default|GetDoor)) _rotation) false false)
        (Variables|Default|SetDoorOpen true)))))

(event EventBeginPlay)

(event Collision|EventActorBeginOverlap
  (params (OtherActor :type Actor%20Object%20Reference)))

(event EventTick
  (params (DeltaSeconds :type Float%20%28single-precision%29)))

(fn ConstructionScript)