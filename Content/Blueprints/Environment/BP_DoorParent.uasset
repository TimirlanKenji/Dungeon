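; BP_DoorParent is a base door actor that swings its Frame component open and closed.
; OpenDoor plays the DoorOpenSwing timeline to rotate the frame by 90 degrees, but only while the player character's max walk speed is below 200.
; CloseDoor reverses the same timeline without that check.
; An unconnected SwingOpen branch for direction-based opening and a DoorOpen flag never runs.
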(event Custom|OpenDoor
  (if (not (>= (Variables|/Script/Engine.CharacterMovementComponent|GetMaxWalkSpeed (Variables|/Script/Engine.Character|GetCharacterMovement (.AsBP%20Third%20Person%20Character (Utilities|Casting|CastToBP_ThirdPersonCharacter (Game|GetPlayerCharacter 0))))) 2e+02))
    (bind _alpha (Timeline|DoorOpenSwing Play)
      (:Update
        (Transformation|SetRelativeRotation (Variables|Default|GetFrame) (Math|Rotator|Lerp(Rotator) "0, 0, 0" "0,-90.000000, 0" _alpha) false false)))))

(event Custom|CloseDoor
  (bind _alpha (Timeline|DoorOpenSwing Reverse)
    (:Update
      (Transformation|SetRelativeRotation (Variables|Default|GetFrame) (Math|Rotator|Lerp(Rotator) "0, 0, 0" "0,-90.000000, 0" _alpha) false false))))

(event EventBeginPlay)

(event Collision|EventActorBeginOverlap
  (params (OtherActor :type Actor%20Object%20Reference)))

(event EventTick
  (params (DeltaSeconds :type Float%20%28single-precision%29)))

(fn ConstructionScript)