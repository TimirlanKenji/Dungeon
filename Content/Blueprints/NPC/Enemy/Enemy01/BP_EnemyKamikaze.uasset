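; Kamikaze enemy that chases the third-person player and explodes on contact, dealing damage.
; PawnSensing triggers an AI move toward any BP_ThirdPersonCharacter it sees.
; Capsule overlap with that character destroys the enemy, then spawns an explosion effect and sound at player 0's location.
; It passes its Damage to player 0's DamageSum and calls PlayerDamaged.
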(event OnComponentBeginOverlap(CapsuleComponent)
  (params (OverlappedComponent :type Primitive%20Component%20Object%20Reference) (OtherActor :type Actor%20Object%20Reference) (OtherComp :type Primitive%20Component%20Object%20Reference) (OtherBodyIndex :type Integer) (bFromSweep :type Boolean) (SweepResult :type Hit%20Result%20Structure%20%28by%20ref%29))
  (bind _returnvalue (Game|GetPlayerCharacter 0))
  (bind _returnvalue_2 (Transformation|GetActorLocation _returnvalue))
  (Utilities|Casting|CastToBP_ThirdPersonCharacter OtherActor)
  (Actor|DestroyActor)
  (Effects|SpawnEmitteratLocation "/Game/AdvancedMagicFX13/Particles/P_ky_explosion1.P_ky_explosion1" _returnvalue_2 "0, 0, 0" "2.000000,2.000000,2.000000")
  (Audio|PlaySoundatLocation "/Game/Music/Explosion.Explosion" _returnvalue_2 "0, 0, 0" 1.0 1.0 0.0 0 0 0)
  (bind _asbp_third_person_character (Utilities|Casting|CastToBP_ThirdPersonCharacter (Game|GetPlayerCharacter 0)))
  (Variables|/Game/Blueprints/BP_ThirdPersonCharacter.BP_ThirdPersonCharacter_C|SetDamageSum _asbp_third_person_character (Variables|Default|GetDamage))
  (Default|PlayerDamaged _asbp_third_person_character))

(event OnSeePawn(PawnSensing)
  (params (Pawn :type Pawn%20Object%20Reference))
  (bind _asbp_third_person_character (Utilities|Casting|CastToBP_ThirdPersonCharacter Pawn))
  (AI|AIMoveTo self "0, 0, 0" _asbp_third_person_character 5.0 false))

(event EventBeginPlay)

(event Collision|EventActorBeginOverlap
  (params (OtherActor :type Actor%20Object%20Reference)))

(event EventTick
  (params (DeltaSeconds :type Float%20%28single-precision%29)))

(fn ConstructionScript
  (|CallParentFunction))