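; Trigger volume that loads and unloads lists of named streaming levels when anything overlaps its box, whose extent is set in the construction script.
; Overlap starts the load chain, then the unload chain, each advancing through its name array by re-invoking a custom event after each latent stream call and resetting its index at the end.
; Loads are blocking and made visible, while unloads are non-blocking.
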(event OnComponentBeginOverlap(Box)
  (params (OverlappedComponent :type Primitive%20Component%20Object%20Reference) (OtherActor :type Actor%20Object%20Reference) (OtherComp :type Primitive%20Component%20Object%20Reference) (OtherBodyIndex :type Integer) (bFromSweep :type Boolean) (SweepResult :type Hit%20Result%20Structure%20%28by%20ref%29))
  (Utilities|FlowControl|Sequence
    (:then_0
      (if (< (Variables|Default|GetCurrentLoadlevelID) (Utilities|Array|Length (Variables|Default|GetLevelsToLoadNames)))
        (bind _output_get (Variables|Default|SetCurrentLevelToLoad (Utilities|Array|Get(acopy) (Variables|Default|GetLevelsToLoadNames) (Variables|Default|GetCurrentLoadlevelID))))
        (Game|LoadStreamLevel(byName) _output_get true true)
        (CallFunction|LoadNextLevel)
        (else
          (Variables|Default|SetCurrentLoadlevelID 0))))
    (:then_1
      (if (< (Variables|Default|GetCurrentUnloadlevelID) (Utilities|Array|Length (Variables|Default|GetLevelsToUnloadNames)))
        (bind _output_get_2 (Variables|Default|SetCurrentLevelToUnload (Utilities|Array|Get(acopy) (Variables|Default|GetLevelsToUnloadNames) (Variables|Default|GetCurrentUnloadlevelID))))
        (Game|UnloadStreamLevel(byName) _output_get_2 false)
        (CallFunction|UnloadNextLevel)
        (else
          (Variables|Default|SetCurrentUnloadlevelID 0))))))

(event Custom|UnloadNextLevel
  (Math|Integer|IncrementInt (Variables|Default|GetCurrentUnloadlevelID)
    (:%20%20
      (if (< (Variables|Default|GetCurrentUnloadlevelID) (Utilities|Array|Length (Variables|Default|GetLevelsToUnloadNames)))
        (bind _output_get (Variables|Default|SetCurrentLevelToUnload (Utilities|Array|Get(acopy) (Variables|Default|GetLevelsToUnloadNames) (Variables|Default|GetCurrentUnloadlevelID))))
        (Game|UnloadStreamLevel(byName) _output_get false)
        (CallFunction|UnloadNextLevel)
        (else
          (Variables|Default|SetCurrentUnloadlevelID 0))))))

(event Custom|LoadNextLevel
  (Math|Integer|IncrementInt (Variables|Default|GetCurrentLoadlevelID)
    (:%20%20
      (if (< (Variables|Default|GetCurrentLoadlevelID) (Utilities|Array|Length (Variables|Default|GetLevelsToLoadNames)))
        (bind _output_get (Variables|Default|SetCurrentLevelToLoad (Utilities|Array|Get(acopy) (Variables|Default|GetLevelsToLoadNames) (Variables|Default|GetCurrentLoadlevelID))))
        (Game|LoadStreamLevel(byName) _output_get true true)
        (CallFunction|LoadNextLevel)
        (else
          (Variables|Default|SetCurrentLoadlevelID 0))))))

(event EventBeginPlay)

(fn ConstructionScript
  (Components|Box|SetBoxExtent (Variables|Default|GetBox) (Variables|Default|GetExtent) true))

(fn OnLevelLoaded)